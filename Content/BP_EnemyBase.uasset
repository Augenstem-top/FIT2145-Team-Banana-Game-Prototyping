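; BP_EnemyBase is an enemy Blueprint, named as a base, that tracks health and swaps sprite flipbooks for walking and death.
; On BeginPlay it shows the walk flipbook and fills current HP from max HP.
; TakeDamage subtracts from current HP; at zero or below it disables collision, switches to the death flipbook and destroys the actor after a short fixed delay.
; It contains no movement or attack logic.
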(event `self.ReceiveBeginPlay`
  (`PaperFlipbookComponent.SetFlipbook` (`self.EnemySprite`) (`self.WalkFlipbook`))
  (set `self.CurrentHP` (`self.MaxHP`)))

(event `TakeDamage`
  (params (DamageAmount :type "Float (double-precision)"))
  (bind _output_get (set `self.CurrentHP` (- (`self.CurrentHP`) DamageAmount)))
  (if (<= _output_get 0.0)
    (`self.SetActorEnableCollision` false)
    (`PaperFlipbookComponent.SetFlipbook` (`self.EnemySprite`) (`self.DeathFlipbook`))
    (`KismetSystemLibrary.Delay` 0.5)
    (`self.K2_DestroyActor`)))

(fn `UserConstructionScript`)